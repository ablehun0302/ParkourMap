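; BP_Monster is a monster that wanders in random directions and chases the player when within detection range.
; Each Tick it feeds MoveDirection into AddMovementInput, then updates that direction from the distance to player pawn 0.
; In range, the direction becomes the unnormalized vector toward the player.
; Out of range, a delta-time accumulator periodically calls RandomDirection, also run at BeginPlay, to pick a normalized direction with random X and Y.
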(event EventBeginPlay
  (Utilities|RandomDirection))

(event EventTick
  (params (DeltaSeconds :type Float%20%28single-precision%29))
  (Pawn|Input|AddMovementInput (Variables|Default|GetMoveDirection) 1.0 false)
  (if (<= (Transformation|GetDistanceTo (Game|Player|GetPlayerPawn 0)) (Variables|Default|GetDetectDistance))
    ;[0.15 0.15 0.15 0.5] 플레이어 따라가기
    (Variables|Default|SetMoveDirection (- (Transformation|GetActorLocation (Game|Player|GetPlayerPawn 0)) (Transformation|GetActorLocation)))
    (else
      ;[0.15 0.15 0.15 0.5] 랜덤 움직임
      (bind _output_get (Variables|Default|SetTime (+ (Utilities|Time|GetWorldDeltaSeconds) (Variables|Default|GetTime))))
      (if (>= _output_get (Variables|Default|GetChangeDirInterval))
        (Utilities|RandomDirection)
        (Variables|Default|SetTime 0.0)))))

(fn ConstructionScript)